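; Level process controller for the PushBox game that shows the pending transition screen when a level finishes.
; On BeginPlay it binds to the OnPendingTransitionStarted event.
; When that fires, it creates the pending widget, passing itself and the first player controller, and adds it to the viewport.
; It then switches input to UI only with the widget focused and shows the mouse cursor.
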(event Custom|CurrentLevelFinished
  (params (bLevelPassed :type Boolean) (CurrentIndex :type Integer) (CurrentLevelId :type Name))
  (bind _returnvalue (Game|GetPlayerController 0))
  (bind _returnvalue_2 (UserInterface|CreateWidget (Variables|Default|GetPendingWidgetClass) (Game|GetPlayerController 0) self (Game|GetPlayerController 0)))
  (bind _output_get (Variables|Default|SetPendingWidget _returnvalue_2))
  (UserInterface|Viewport|AddtoViewport _output_get 0)
  (Input|SetInputModeUIOnly _returnvalue (Variables|Default|GetPendingWidget) "DoNotLock" false)
  (Variables|/Script/Engine.PlayerController|SetbShowMouseCursor _returnvalue true))

(event EventBeginPlay
  (EventDispatchers|BindEventtoOnPendingTransitionStarted (delegate Custom|CurrentLevelFinished)))

(event Collision|EventActorBeginOverlap
  (params (OtherActor :type Actor%20Object%20Reference)))

(event EventTick
  (params (DeltaSeconds :type Float%20%28single-precision%29)))

(fn ConstructionScript)