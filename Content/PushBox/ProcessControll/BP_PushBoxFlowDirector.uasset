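; BP_PushBoxFlowDirector is the flow director Blueprint for the PushBox game, showing UI at level transitions and at the end of the flow.
; On BeginPlay it binds handlers to its pending-transition-started and flow-completed events.
; A transition creates a pending widget that receives the director as FlowDirector and is added to the viewport.
; Flow completion creates and displays a finish widget for the first player controller.
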(event Custom|TransitionStarted
  (params (bLevelPassed :type Boolean) (CurrentIndex :type Integer) (CurrentLevelId :type Name))
  (bind _returnvalue (Game|GetPlayerController 0))
  (bind _returnvalue_2 (UserInterface|CreateWidget (Variables|Default|GetPendingWidgetClass) _returnvalue _returnvalue self))
  (UserInterface|Viewport|AddtoViewport _returnvalue_2 0))

(event Custom|FlowCompleted
  (bind _returnvalue (Game|GetPlayerController 0))
  (bind _returnvalue_2 (UserInterface|CreateWidget (Variables|Default|GetFinishWidgetClass) _returnvalue _returnvalue))
  (UserInterface|Viewport|AddtoViewport _returnvalue_2 0))

(event EventBeginPlay
  (EventDispatchers|BindEventtoOnPendingTransitionStarted (delegate Custom|TransitionStarted))
  (EventDispatchers|BindEventtoOnFlowCompleted (delegate Custom|FlowCompleted)))

(event Collision|EventActorBeginOverlap
  (params (OtherActor :type Actor%20Object%20Reference)))

(event EventTick
  (params (DeltaSeconds :type Float%20%28single-precision%29)))

(fn ConstructionScript)